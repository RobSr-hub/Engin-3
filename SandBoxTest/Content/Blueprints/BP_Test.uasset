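; Test actor that prints debug messages to check collision and overlap events on its cube components.
; Tick prints real time seconds, Cube_3 logs begin overlaps, and Cube_1 and Cube_2 log hits in distinct colors with French messages.
; Cube_1 builds its message with string Append while the other cubes use FormatText, and each print has its own key so messages update in place.
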(event `self.ReceiveBeginPlay`
  ; Test Print
)

(event `self.ReceiveTick`
  (params (DeltaSeconds :type "Float (single-precision)"))
  ; Test Print
  (`KismetSystemLibrary.PrintText` (`KismetTextLibrary.Conv_DoubleToText` (`GameplayStatics.GetRealTimeSeconds`) "HalfToEven") true true (struct :`G` 0.66 :`B` 1.0 :`A` 1.0) 2.0 "TagKey"))

(event `self.Cube_3.OnComponentBeginOverlap`
  (params (OverlappedComponent :type "PrimitiveComponent Object Reference") (OtherActor :type "Actor Object Reference") (OtherComp :type "PrimitiveComponent Object Reference") (OtherBodyIndex :type Integer) (bFromSweep :type Boolean) (SweepResult :type "HitResult Structure (by ref)"))
  (`KismetSystemLibrary.PrintText` (`|FormatText` "{0} Overlap avec le {1}" OtherComp OverlappedComponent) true true (struct :`G` 0.66 :`B` 1.0 :`A` 1.0) 2.0 "LogOverlap"))

(event `self.Cube_1.OnComponentHit`
  (params (HitComponent :type "PrimitiveComponent Object Reference") (OtherActor :type "Actor Object Reference") (OtherComp :type "PrimitiveComponent Object Reference") (NormalImpulse :type "Vector Structure") (Hit :type "HitResult Structure (by ref)"))
  ; Test Collisions
  (`KismetSystemLibrary.PrintString` (`KismetStringLibrary.Concat_StrStr` "L'objet " (`KismetTextLibrary.Conv_TextToString` (`KismetTextLibrary.Conv_ObjectToText` (`self.Cube_1`))) " collisionne avec" (`KismetSystemLibrary.GetDisplayName` OtherComp)) true true (struct :`R` 1.0 :`B` 0.718639 :`A` 1.0) 2.0 "LogHit"))

(event `self.Cube_2.OnComponentHit`
  (params (HitComponent :type "PrimitiveComponent Object Reference") (OtherActor :type "Actor Object Reference") (OtherComp :type "PrimitiveComponent Object Reference") (NormalImpulse :type "Vector Structure") (Hit :type "HitResult Structure (by ref)"))
  ; Test Collisions
  (`KismetSystemLibrary.PrintText` (`|FormatText` "l'objet {0} collisionne avec {1}" (`self.Cube_2`) OtherComp) true true (struct :`R` 1.0 :`G` 0.966449 :`A` 1.0) 2.0 "LogHit_2"))

(fn `UserConstructionScript`)